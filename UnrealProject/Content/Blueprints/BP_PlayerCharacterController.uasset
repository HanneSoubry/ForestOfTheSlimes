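; Player controller that moves BP_PlayerCharacter along world X/Y axes and turns it toward its movement direction.
; Each Tick normalizes the combined axis input, scales it by MaxWalkSpeed and writes it straight to CharacterMovement velocity, bypassing AddMovementInput.
; Stored rotation holds the facing while idle or attacking, and attacking also skips the velocity update.
; Mouse-cursor aiming and aim-target spawning are present but disconnected.
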(event `InputAxis|MovementForward`
  (params (AxisValue :type "Float (single-precision)"))
  ;[1 1 1] Handle movement input
  (set `self.ForwardVector` (`KismetMathLibrary.MakeVector` AxisValue)))

(event `InputAxis|MovementRight`
  (params (AxisValue :type "Float (single-precision)"))
  ;[1 1 1] Handle movement input
  (set `self.RightVector` (`KismetMathLibrary.MakeVector` 0.0 AxisValue)))

(event `self.ReceiveTick`
  (params (DeltaSeconds :type "Float (single-precision)"))
  (bind _currentdirection (`self.CurrentDirection`))
  ;[1 0 0] Tick Event
  (bind _asbp_player_character (cast `/Game/Blueprints/BP_PlayerCharacter` (`self.K2_GetPawn`)))
  (if (`/Game/Blueprints/BP_PlayerCharacter.IsAttacking` _asbp_player_character)
    ;[1 1 1] if attacking, don't move, keep current rotation
    (`self.SetControlRotation` (`self.CurrentRotation`))
    (else
      ;[1 1 1] Calculate Velocity
      ;;[1 1 1] set direction to length 1 (avoid diagonal speed bonus) & mulitply with speed
      (bind _output_get (set `self.CurrentDirection` (+ (`self.ForwardVector`) (`self.RightVector`))))
      (`KismetMathLibrary.Vector_Normalize` _output_get)
      (bind _charactermovement (`Character.CharacterMovement` _asbp_player_character))
      (bind _output_get_2 (set `self.CurrentDirection` (* _output_get (`CharacterMovementComponent.MaxWalkSpeed` _charactermovement))))
      (bind _output_get_3 (set `MovementComponent.Velocity` _output_get_2 _charactermovement))
      ;[1 1 1] Calculate Rotation
      ;;[1 1 1] If moving
      (if (> (`KismetMathLibrary.VSize` _output_get_3) 0.0)
        (`self.SetControlRotation` (`KismetMathLibrary.MakeRotFromXY` _currentdirection _currentdirection))
        ;;[1 1 1] Store current rotation (needed if stop moving)
        (set `self.CurrentRotation` (`self.K2_GetActorRotation` (`self.K2_GetPawn`)))
        (else
          (`self.SetControlRotation` (`self.CurrentRotation`)))))))

(event `self.ReceiveBeginPlay`
  ;[1 0 0] BeginPlay Event
  ;[1 1 1] Find initial rotation
  (set `self.CurrentRotation` (`self.K2_GetActorRotation` (`self.K2_GetPawn`))))

(event `InputAxisKey|MouseX`
  (params (AxisValue :type "Float (single-precision)"))
  (`|ExecutionSequence` :!label _label))

(event `InputAxisKey|MouseY`
  (params (AxisValue :type "Float (single-precision)"))
  (goto _label))

(fn `UserConstructionScript`)