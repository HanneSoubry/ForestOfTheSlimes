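; BP_Water is a water area that cleans slime off the player and lowers their sickness.
; Every Tick it polls its Sphere for overlapping player characters, resetting slime and reducing normal slime sickness by SlimeDecrease through the Health component.
; The first detection on each instance notifies BP_SlimeGameMode for the water tutorial.
; Sphere begin and end overlap events start and stop the player's water footsteps audio.
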(event `self.ReceiveTick`
  (params (DeltaSeconds :type "Float (single-precision)"))
  ;[1 1 1] Find overlapping Player
  (for _array_element (`PrimitiveComponent.GetOverlappingActors` (`self.Sphere`) "/Game/Blueprints/BP_PlayerCharacter.BP_PlayerCharacter_C")
    (bind _asbp_player_character (cast `/Game/Blueprints/BP_PlayerCharacter` _array_element))
    (if (`self.First enter`)
      ;[1 1 1] First water tutorial
      (bind _asbp_slime_game_mode (cast `/Game/Blueprints/BP_SlimeGameMode` (`GameplayStatics.GetGameMode`)))
      (`/Game/Blueprints/BP_SlimeGameMode.FirstWaterEntered` _asbp_slime_game_mode)
      (set `self.First enter` false))
    (`/Game/Blueprints/BP_PlayerCharacter.ResetSlime` _asbp_player_character)
    ;[1 1 1] Amount -1 -> decrease sickness
    (`HealthComponent.UpdateSickness` (`/Game/Blueprints/BP_PlayerCharacter.Health` _asbp_player_character) (* (`self.SlimeDecrease`) -1) 0)))

(event `self.Sphere.OnComponentBeginOverlap`
  (params (OverlappedComponent :type "PrimitiveComponent Object Reference") (OtherActor :type "Actor Object Reference") (OtherComp :type "PrimitiveComponent Object Reference") (OtherBodyIndex :type Integer) (bFromSweep :type Boolean) (SweepResult :type "HitResult Structure (by ref)"))
  ;[1 1 1] Sound
  (bind _asbp_player_character (cast `/Game/Blueprints/BP_PlayerCharacter` OtherActor))
  (`AudioComponent.Play` (`/Game/Blueprints/BP_PlayerCharacter.Audio WaterFootsteps` _asbp_player_character) 0.0))

(event `self.Sphere.OnComponentEndOverlap`
  (params (OverlappedComponent :type "PrimitiveComponent Object Reference") (OtherActor :type "Actor Object Reference") (OtherComp :type "PrimitiveComponent Object Reference") (OtherBodyIndex :type Integer))
  ;[1 1 1] Sound
  (bind _asbp_player_character (cast `/Game/Blueprints/BP_PlayerCharacter` OtherActor))
  (`AudioComponent.Stop` (`/Game/Blueprints/BP_PlayerCharacter.Audio WaterFootsteps` _asbp_player_character)))

(fn `UserConstructionScript`)