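; Slime game mode that manages saving, level UI, player respawn and wall progression.
; On BeginPlay it loads or creates the save object, shows the start menu or HUD by level name, and caches requirement walls and enemy spawners.
; Kill counts are forwarded to every wall and wall-down IDs to every spawner.
; The HUD is cached only in Level0, so first-kill and first-water tutorial texts play only there.
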(event `self.ReceiveBeginPlay`
  ;[1 1 1] Try to load SaveGame
  (bind _returnvalue (`GameplayStatics.LoadGameFromSlot` (`self.SaveGameName`) (`self.SaveGameIndex`)))
  (bind _asbp_slime_save_game (cast `/Game/Blueprints/BP_SlimeSaveGame` _returnvalue)
    (:`then`
      (set `self.SaveGameInstance` _asbp_slime_save_game))
    (:`CastFailed`
      ;[1 1 1] Create new SaveGame Instance
      (bind _returnvalue_2 (`GameplayStatics.CreateSaveGameObject` "/Game/Blueprints/BP_SlimeSaveGame.BP_SlimeSaveGame_C"))
      (set `self.SaveGameInstance` _returnvalue_2)))
  (bind _returnvalue_3 (`GameplayStatics.GetCurrentLevelName` true))
  (if (`KismetStringLibrary.EqualEqual_StrStr` _returnvalue_3 "Menu")
    ;[1 1 1] Setup Menu
    (bind _returnvalue_4 (`|CreateWidget` "/Game/Blueprints/BPW_StartMenu.BPW_StartMenu_C"))
    (`UserWidget.AddToViewport` _returnvalue_4 0)
    (else
      ;[1 1 1] Setup level Hud
      (bind _returnvalue_5 (`|CreateWidget` "/Game/Blueprints/BPW_HUD.BPW_Hud_C"))
      (`UserWidget.AddToViewport` _returnvalue_5 0)
      ;[1 1 1] Cache HUD
      (bind _returnvalue_6 (`GameplayStatics.GetCurrentLevelName` true))
      (if (`KismetStringLibrary.EqualEqual_StrStr` _returnvalue_6 "Level0")
        (set `self.HudInstance` _returnvalue_5))
      ;[1 1 1] Find requirement walls
      (bind _outactors (`GameplayStatics.GetAllActorsOfClass` "/Game/Blueprints/BP_RequirementWall.BP_RequirementWall_C"))
      (set `self.RequirementWalls` _outactors)
      ;[1 1 1] Find requirement walls
      (bind _outactors_2 (`GameplayStatics.GetAllActorsOfClass` "/Game/Blueprints/BP_EnemySpawner.BP_EnemySpawner_C"))
      (set `self.EnemySpawners` _outactors_2))))

(event `Save Game`
  ;[1 1 1] Save Game
  (`GameplayStatics.SaveGameToSlot` (`self.SaveGameInstance`) (`self.SaveGameName`) (`self.SaveGameIndex`)))

(event `FirstSlimeKilled`
  ;[1 1 1] Start tutorial
  (bind _hudinstance (`self.HudInstance`)
    (:`then`
      (`/Game/Blueprints/BPW_HUD.StartSlimeText` _hudinstance))
    (:`else`)))

(event `RespawnPlayer`
  (bind _returnvalue (`GameplayStatics.GetPlayerController` 0))
  ;[1 1 1] Respawn player
  (bind _returnvalue_2 (`|SpawnActorFromClass` (`self.DefaultPawnClass`) (`self.GetTransform` (`self.K2_FindPlayerStart` _returnvalue)) "Undefined" "OverrideRootScale" null null))
  (`Controller.Possess` _returnvalue _returnvalue_2))

(event `FirstWaterEntered`
  ;[1 1 1] Start tutorial
  (bind _hudinstance (`self.HudInstance`)
    (:`then`
      (`/Game/Blueprints/BPW_HUD.StartWaterText` _hudinstance))
    (:`else`)))

(event `IncreaseKillCount`
  (params (Amount :type Integer))
  ;[1 1 1] Increase Kill Count
  (for _array_element (`self.RequirementWalls`)
    (`/Game/Blueprints/BP_RequirementWall.DecreaseSlime` _array_element Amount)))

(event `WallDown`
  (params (ID :type Integer))
  ;[1 1 1] Check wall down for all spawners
  (for _array_element (`self.EnemySpawners`)
    (`/Game/Blueprints/BP_EnemySpawner.WallDown` _array_element ID)))

(fn `UserConstructionScript`)