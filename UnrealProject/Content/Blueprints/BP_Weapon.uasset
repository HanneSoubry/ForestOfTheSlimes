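; BP_Weapon is a weapon actor that kills slimes it touches while attacking and tallies what it collects.
; On overlap during an attack, it increments a normal or poison counter by the living slime's type, counting shooting slimes as normal, then calls KillSlime.
; ConsumeSlime caches both counters, resets them to zero and returns the cached amounts to the caller.
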(event `self.ReceiveActorBeginOverlap`
  (params (OtherActor :type "Actor Object Reference"))
  (if (`self.Attacking`)
    (bind _asbp_base_slime (cast `/Game/Blueprints/BP_BaseSlime` OtherActor))
    ;[1 1 1] if not dead yet
    (if (not (`/Game/Blueprints/BP_BaseSlime.IsDead` _asbp_base_slime))
      ;[1 1 1] Remember slime
      (switch `/Game/Blueprints/Enum_SlimeType` (`/Game/Blueprints/BP_BaseSlime.SlimeType` _asbp_base_slime)
        (:`NewEnumerator0`
          ;;[1 1 1] Shooting = other behavior, same normal slime
          (set `self.SlimeAmountNormal` (+ (`self.SlimeAmountNormal`) 1) :!label _label))
        (:`NewEnumerator1`
          (set `self.SlimeAmountPoison` (+ (`self.SlimeAmountPoison`) 1)))
        (:`NewEnumerator2`
          (goto _label)))
      (`/Game/Blueprints/BP_BaseSlime.KillSlime` _asbp_base_slime))))

(fn `ConsumeSlime`
  (returns (SlimeNormal :type Integer) (SlimePoison :type Integer))
  (locals (SlimeNormalOutput :type Integer) (SlimePoisonOutput :type Integer))
  (`|ExecutionSequence`
    (:`then_0`
      ;[1 1 1] Cache slime
      (set `local.SlimeNormalOutput` (`self.SlimeAmountNormal`))
      ;[1 1 1] Reset slime
      (set `self.SlimeAmountNormal` 0))
    (:`then_1`
      (set `local.SlimePoisonOutput` (`self.SlimeAmountPoison`))
      (set `self.SlimeAmountPoison` 0))
    (:`then_2`
      ;[1 1 1] Pass cached amount to other object
      (return (`local.SlimeNormalOutput`) (`local.SlimePoisonOutput`)))))

(fn `UserConstructionScript`)