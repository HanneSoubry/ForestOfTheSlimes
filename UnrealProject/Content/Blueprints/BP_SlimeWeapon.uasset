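; BP_SlimeWeapon is a projectile that flies along its spawn facing and damages the player on contact.
; Tick moves it with swept location updates until it overlaps anything other than a BP_SlimeShoothing, the shooting slime.
; The overlap hides the sphere, plays impact sound and particles, and calls DoDamage on the player's Health.
; After a hit it stops moving and destroys itself once a timer expires.
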(event `self.ReceiveBeginPlay`
  (`self.SetActorEnableCollision` true)
  ;[1 1 1] Set initial Direction
  (set `self.Direction` (`KismetMathLibrary.Normal` (`KismetMathLibrary.GetForwardVector` (`self.K2_GetActorRotation`)))))

(event `self.ReceiveTick`
  (params (DeltaSeconds :type "Float (single-precision)"))
  (if (not (`self.Hit`))
    ;[1 1 1] Move
    (`self.K2_SetActorLocation` (+ (`self.K2_GetActorLocation`) (* (`self.Direction`) (* DeltaSeconds (`self.Speed`)))) true)
    (else
      ;[1 1 1] Destroy if timer expired
      (bind _output_get (set `self.Timer` (+ DeltaSeconds (`self.Timer`))))
      (if (>= _output_get (`self.MaxTimer`))
        (`self.K2_DestroyActor`)))))

(event `self.ReceiveActorBeginOverlap`
  (params (OtherActor :type "Actor Object Reference"))
  (bind _sphere (`self.Sphere`))
  ;[1 1 1] If anything (except shooting slime)  hit, explode
  (cast `/Game/Blueprints/BP_SlimeShoothing` OtherActor
    (:`CastFailed`
      (`SceneComponent.SetVisibility` (`self.Sphere`) false false)
      (set `self.Hit` true)
      (`GameplayStatics.PlaySoundAtLocation` "/Game/Audio/S_SlimeAttack.S_SlimeAttack" (`self.K2_GetActorLocation` OtherActor) (struct) 1.0 1.0 0.0 null null null)
      (`GameplayStatics.SpawnEmitterAtLocation` "/Game/Particles/P_SlimeExplosionGreenSmall.P_SlimeExplosionGreenSmall" (`SceneComponent.K2_GetComponentLocation` _sphere) (`SceneComponent.K2_GetComponentRotation` _sphere) (0.5 0.5 0.5))
      ;[1 1 1] if player hit, do damage
      (bind _asbp_player_character (cast `/Game/Blueprints/BP_PlayerCharacter` OtherActor))
      (`HealthComponent.DoDamage` (`/Game/Blueprints/BP_PlayerCharacter.Health` _asbp_player_character) (`self.Damage`)))))

(event `self.ReceiveActorEndOverlap`
  (params (OtherActor :type "Actor Object Reference"))
  (cast `/Game/Blueprints/BP_SlimeShoothing` OtherActor)
  (`self.SetActorEnableCollision` true))

(fn `UserConstructionScript`)