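; BP_SlimeShoothing is the green, ranged variant of a parent slime Blueprint, setting its own materials, type and kill particle on BeginPlay.
; A sphere overlap with the player character starts or stops the inherited attack behavior.
; The Attack override spawns a BP_SlimeWeapon at the slime, aimed at the targeted player.
; Tick turns the slime toward player 0 without pitching.
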(event `self.ReceiveBeginPlay`
  (bind _staticmesh (`self.StaticMesh`))
  ;[1 1 1] Change color
  (`PrimitiveComponent.SetMaterial` _staticmesh 0 "/Game/Materials/Slime/MI_SlimeGreen.MI_SlimeGreen")
  (`PrimitiveComponent.SetMaterial` _staticmesh 2 "/Game/Materials/Slime/MI_SlimeGreenDetails.MI_SlimeGreenDetails")
  ;[1 1 1] Change slime type
  (set `self.SlimeType` "NewEnumerator2")
  ;[1 1 1] Change Particles
  (set `self.KillParticle` "/Game/Particles/P_SlimeExplosionGreen.P_SlimeExplosionGreen"))

(event `self.Attack`
  (bind _returnvalue (`self.K2_GetActorLocation`))
  ;[1 1 1] Attack function
  (bind _playertoattack (`self.PlayerToAttack`)
    (:`then`
      (`|SpawnActorFromClass` "/Game/Blueprints/BP_SlimeWeapon.BP_SlimeWeapon_C" (`KismetMathLibrary.MakeTransform` _returnvalue (`KismetMathLibrary.FindLookAtRotation` _returnvalue (`self.K2_GetActorLocation` _playertoattack))) "AlwaysSpawn" "OverrideRootScale" null null))
    (:`else`)))

(event `self.ReceiveTick`
  (params (DeltaSeconds :type "Float (single-precision)"))
  (bind (_returnvalue_roll _returnvalue_pitch _returnvalue_yaw) (`KismetMathLibrary.BreakRotator` (`KismetMathLibrary.FindLookAtRotation` (`self.K2_GetActorLocation`) (`self.K2_GetActorLocation` (`GameplayStatics.GetPlayerCharacter` 0)))))
  ;[1 1 1] Rotate to player
  (`self.K2_SetActorRotation` (`KismetMathLibrary.MakeRotator` _returnvalue_roll 0.0 _returnvalue_yaw)))

(event `self.Sphere.OnComponentBeginOverlap`
  (params (OverlappedComponent :type "PrimitiveComponent Object Reference") (OtherActor :type "Actor Object Reference") (OtherComp :type "PrimitiveComponent Object Reference") (OtherBodyIndex :type Integer) (bFromSweep :type Boolean) (SweepResult :type "HitResult Structure (by ref)"))
  (bind _asbp_player_character (cast `/Game/Blueprints/BP_PlayerCharacter` OtherActor))
  (`self.StartAttacking` _asbp_player_character))

(event `self.Sphere.OnComponentEndOverlap`
  (params (OverlappedComponent :type "PrimitiveComponent Object Reference") (OtherActor :type "Actor Object Reference") (OtherComp :type "PrimitiveComponent Object Reference") (OtherBodyIndex :type Integer))
  (cast `/Game/Blueprints/BP_PlayerCharacter` OtherActor)
  (`self.StopAttacking`))

(fn `UserConstructionScript`
  (`parent.UserConstructionScript`))