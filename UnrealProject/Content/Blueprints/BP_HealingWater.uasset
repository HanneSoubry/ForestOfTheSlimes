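; BP_HealingWater is a water actor that heals player characters within its sphere.
; On BeginPlay it calls the parent logic and applies the healing water material to its mesh.
; Each Tick it polls the Sphere for overlapping BP_PlayerCharacter actors, rather than using overlap events, and calls HealOverTime on their Health with HealingRate, without passing DeltaSeconds.
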(event `self.ReceiveBeginPlay`
  (`parent.ReceiveBeginPlay`)
  (`PrimitiveComponent.SetMaterial` (`self.Mesh`) 0 "/Game/Materials/Water/M_HealingWater.M_HealingWater"))

(event `self.ReceiveTick`
  (params (DeltaSeconds :type "Float (single-precision)"))
  (`parent.ReceiveTick` DeltaSeconds)
  (for _array_element (`PrimitiveComponent.GetOverlappingActors` (`self.Sphere`) "/Game/Blueprints/BP_PlayerCharacter.BP_PlayerCharacter_C")
    (bind _asbp_player_character (cast `/Game/Blueprints/BP_PlayerCharacter` _array_element))
    ;[1 1 1] Heal
    (`HealthComponent.HealOverTime` (`/Game/Blueprints/BP_PlayerCharacter.Health` _asbp_player_character) (`self.HealingRate`))))

(fn `UserConstructionScript`
  (`parent.UserConstructionScript`))