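; Poisonous slime Blueprint, a child variant of a parent slime class with a purple look.
; On BeginPlay it swaps two mesh materials to purple, sets the slime type enum and replaces the kill particle with a purple explosion.
; It does not call the parent BeginPlay, and the construction script only runs the parent's.
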(event `self.ReceiveBeginPlay`
  (bind _staticmesh (`self.StaticMesh`))
  ;[1 1 1] Change color
  (`PrimitiveComponent.SetMaterial` _staticmesh 0 "/Game/Materials/Slime/MI_SlimePurple.MI_SlimePurple")
  (`PrimitiveComponent.SetMaterial` _staticmesh 2 "/Game/Materials/Slime/MI_SlimePurpleDetails.MI_SlimePurpleDetails")
  ;[1 1 1] Change slime type
  (set `self.SlimeType` "NewEnumerator1")
  ;[1 1 1] Change Particles
  (set `self.KillParticle` "/Game/Particles/P_SlimeExplosionPurple.P_SlimeExplosionPurple"))

(fn `UserConstructionScript`
  (`parent.UserConstructionScript`))