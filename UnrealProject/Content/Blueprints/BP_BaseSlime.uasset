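; BP_BaseSlime is a slime enemy character that attacks the player at close range and dies in one hit.
; AttackBox overlap with the player starts a looping Attack timer, stopped when an overlap ends.
; Each attack deals damage immediately, then Tick drives a horizontal lunge out and back via unswept location changes while CharacterMovement is deactivated.
; KillSlime squashes the mesh, plays effects, disables collision and destroys the actor after a delay.
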(event `self.ReceiveBeginPlay`
  (set `self.KillParticle` "/Game/Particles/P_SlimeExplosionGreen.P_SlimeExplosionGreen"))

(event `KillSlime`
  (bind _staticmesh (`self.StaticMesh`))
  (bind (_returnvalue_x _returnvalue_y _returnvalue_z) (`KismetMathLibrary.BreakVector` (`SceneComponent.K2_GetComponentScale` (`self.StaticMesh`))))
  ;[1 1 1] One-hit kills
  (`/Engine/EditorBlueprintResources/StandardMacros.DoOnce` false
    (:`Completed`
      (`SceneComponent.SetWorldScale3D` (`self.StaticMesh`) (`KismetMathLibrary.MakeVector` _returnvalue_x _returnvalue_y (/ _returnvalue_z 2.0)))
      (`CharacterMovementComponent.DisableMovement` (`self.CharacterMovement`))
      (set `self.IsDead` true)
      (`GameplayStatics.SpawnEmitterAtLocation` (`self.KillParticle`) (`SceneComponent.K2_GetComponentLocation` _staticmesh) (`SceneComponent.K2_GetComponentRotation` _staticmesh))
      (`GameplayStatics.PlaySoundAtLocation` "/Game/Audio/S_SlimeDead.S_SlimeDead" (`self.K2_GetActorLocation`) (struct) 1.0 1.0 0.0 null null null)
      (`KismetSystemLibrary.K2_ClearTimer` null "Attack")
      (`PrimitiveComponent.SetCollisionEnabled` (`self.MeshBox`) "NoCollision")
      (`PrimitiveComponent.SetCollisionEnabled` (`self.AttackBox`) "NoCollision")
      (`PrimitiveComponent.SetCollisionEnabled` (`self.StaticMesh`) "NoCollision")
      (`PrimitiveComponent.SetCollisionEnabled` (`self.CapsuleComponent`) "NoCollision")
      (`KismetSystemLibrary.Delay` 2.0)
      (`self.K2_DestroyActor`))))

(event `StartAttacking`
  (params (`other actor` :type "Actor Object Reference"))
  ;[1 1 1] Attack timer
  (if (not (`self.IsDead`))
    (bind _asbp_player_character (cast `/Game/Blueprints/BP_PlayerCharacter` `other actor`))
    (set `self.PlayerToAttack` _asbp_player_character)
    (`KismetSystemLibrary.K2_SetTimer` null "Attack" (`self.AttackDelay`) true)))

(event `self.AttackBox.OnComponentBeginOverlap`
  (params (OverlappedComponent :type "PrimitiveComponent Object Reference") (OtherActor :type "Actor Object Reference") (OtherComp :type "PrimitiveComponent Object Reference") (OtherBodyIndex :type Integer) (bFromSweep :type Boolean) (SweepResult :type "HitResult Structure (by ref)"))
  ;[1 1 1] Attack timer
  (`self.StartAttacking` OtherActor))

(event `StopAttacking`
  ;[1 1 1] Attack timer
  (`KismetSystemLibrary.K2_ClearTimer` null "Attack"))

(event `self.AttackBox.OnComponentEndOverlap`
  (params (OverlappedComponent :type "PrimitiveComponent Object Reference") (OtherActor :type "Actor Object Reference") (OtherComp :type "PrimitiveComponent Object Reference") (OtherBodyIndex :type Integer))
  ;[1 1 1] Attack timer
  (`self.StopAttacking`))

(event `Attack`
  (bind (_returnvalue_x _returnvalue_y) (`KismetMathLibrary.BreakVector` (`KismetMathLibrary.GetDirectionUnitVector` (`self.K2_GetActorLocation`) (`self.K2_GetActorLocation` (`self.PlayerToAttack`)))))
  ;[1 1 1] Attack function
  (bind _playertoattack (`self.PlayerToAttack`)
    (:`then`
      (`HealthComponent.DoDamage` (`/Game/Blueprints/BP_PlayerCharacter.Health` _playertoattack) (`self.AttackDamage`))
      (set `self.IsAttackingForward` true)
      (`ActorComponent.Deactivate` (`self.CharacterMovement`))
      (set `self.AttackDirection` (`KismetMathLibrary.Normal` (`KismetMathLibrary.MakeVector` _returnvalue_x _returnvalue_y)))
      (set `self.MovementDone` (0.0 0.0 0.0))
      (`GameplayStatics.PlaySoundAtLocation` "/Game/Audio/S_SlimeAttack.S_SlimeAttack" (`self.K2_GetActorLocation`) (struct) 1.0 1.0 0.0 null null null))
    (:`else`)))

(event `self.ReceiveTick`
  (params (DeltaSeconds :type "Float (single-precision)"))
  ;[1 1 1] Update attack move
  (if (or (`self.IsAttackingForward`) (`self.IsAttackingReturn`))
    (bind _done (`self.UpdateAttackMovement` DeltaSeconds))
    (if _done
      (`ActorComponent.Activate` (`self.CharacterMovement`) false))))

(fn `UpdateAttackMovement`
  (params (DeltaSeconds :type "Float (double-precision)"))
  (returns (Done :type Boolean))
  (locals (NewLocalVar_0 :type Boolean))
  (bind _returnvalue (* (`self.AttackDirection`) (* (`self.AttackMoveSpeed`) DeltaSeconds)))
  (bind _returnvalue_2 (* (`self.AttackDirection`) (* DeltaSeconds (`self.AttackMoveSpeed`))))
  (if (`self.IsAttackingForward`)
    (set `self.MovementDone` (+ _returnvalue (`self.MovementDone`)))
    (`self.K2_SetActorLocation` (+ (`self.K2_GetActorLocation`) _returnvalue))
    (if (>= (`KismetMathLibrary.VSize` (`self.MovementDone`)) (`self.AttackLength`))
      (set `self.IsAttackingForward` false)
      (set `self.IsAttackingReturn` true)
      (set `self.MovementDone` (0.0 0.0 0.0)))
    (return false)
    (elif (`self.IsAttackingReturn`)
      (set `self.MovementDone` (+ _returnvalue_2 (`self.MovementDone`)))
      (`self.K2_SetActorLocation` (- (`self.K2_GetActorLocation`) _returnvalue_2))
      (if (>= (`KismetMathLibrary.VSize` (`self.MovementDone`)) (`self.AttackLength`))
        (set `self.IsAttackingForward` false)
        (set `self.IsAttackingReturn` false)
        (return true)
        (else
          (return false))))))

(fn `UserConstructionScript`)