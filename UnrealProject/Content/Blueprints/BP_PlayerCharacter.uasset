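; Player character that attacks with a socket-attached weapon and collects normal and poison slime from its kills.
; After each timed attack it takes the weapon's slime into its totals and reports kills to the game mode, including a one-time first-slime event.
; Each tick, carried slime switches it to run speed and feeds the Health component's sickness until ResetSlime clears it.
; Death disables movement and, after a delay, fails the level through the game state.
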(event `self.ReceiveBeginPlay`
  ;[1 0 0] Event BeginPlay
  (`parent.ReceiveBeginPlay`)
  (`|ExecutionSequence`
    (:`then_0`
      ;[1 1 1] Spawn weapon
      (bind _returnvalue (`|SpawnActorFromClass` "/Game/Blueprints/BP_Weapon.BP_Weapon_C" (`SceneComponent.K2_GetComponentToWorld` (`self.Socket`)) "Undefined" "OverrideRootScale" null null))
      (bind _output_get (set `self.CurrentWeapon` _returnvalue))
      (`self.K2_AttachToComponent` _output_get (`self.Mesh`) "RightHandSocket" "SnapToTarget" "SnapToTarget" "KeepRelative" true))
    (:`then_1`
      ;[1 1 1] Set walk speed
      (set `CharacterMovementComponent.MaxWalkSpeed` (`self.WalkSpeed`) (`self.CharacterMovement`)))))

(event `InputAction|Attack`
  (params (Key :type "Key Structure"))
  ;[1 1 1] Attack
  (:`Pressed`
    (if (not (`self.IsAttacking`))
      (set `self.IsAttacking` true)
      (set `/Game/Blueprints/BP_Weapon.Attacking` true (`self.CurrentWeapon`))
      (`KismetSystemLibrary.Delay` 1.0)
      (set `self.IsAttacking` false)
      (set `/Game/Blueprints/BP_Weapon.Attacking` false (`self.CurrentWeapon`))
      ;[1 1 1] Get slime from weapon
      (bind (_slimenormal _slimepoison) (`/Game/Blueprints/BP_Weapon.ConsumeSlime` (`self.CurrentWeapon`)))
      (`|ExecutionSequence`
        (:`then_0`
          (set `self.SlimeAmountNormal` (+ _slimenormal (`self.SlimeAmountNormal`))))
        (:`then_1`
          (set `self.SlimeAmountPoison` (+ _slimepoison (`self.SlimeAmountPoison`))))
        (:`then_2`
          (bind _asbp_slime_game_mode (cast `/Game/Blueprints/BP_SlimeGameMode` (`GameplayStatics.GetGameMode`)))
          (`/Game/Blueprints/BP_SlimeGameMode.IncreaseKillCount` _asbp_slime_game_mode (+ _slimenormal _slimepoison))
          ;[1 1 1] First slime tutorial
          (if (> (`self.SlimeAmountNormal`) 0)
            (`/Engine/EditorBlueprintResources/StandardMacros.DoOnce` false
              (:`Completed`
                (bind _asbp_slime_game_mode_2 (cast `/Game/Blueprints/BP_SlimeGameMode` (`GameplayStatics.GetGameMode`)))
                (`/Game/Blueprints/BP_SlimeGameMode.FirstSlimeKilled` _asbp_slime_game_mode_2)))))))))

(event `self.Health.OnDeath`
  ;[1 1 1] On death, failed level
  (`CharacterMovementComponent.DisableMovement` (`self.CharacterMovement`))
  (`KismetSystemLibrary.Delay` 2.0)
  (bind _asbp_slime_game_state (cast `/Game/Blueprints/BP_SlimeGameState` (`GameplayStatics.GetGameState`)))
  (`/Game/Blueprints/BP_SlimeGameState.FailedLevel` _asbp_slime_game_state))

(event `ResetSlime`
  ;[1 1 1] Reset Sllime
  (`|ExecutionSequence`
    (:`then_0`
      (set `self.SlimeAmountNormal` 0))
    (:`then_1`
      (set `self.SlimeAmountPoison` 0))
    (:`then_2`
      ;[1 1 1] Reset walk speed
      (set `CharacterMovementComponent.MaxWalkSpeed` (`self.WalkSpeed`) (`self.CharacterMovement`)))))

(event `self.ReceiveTick`
  (params (DeltaSeconds :type "Float (single-precision)"))
  ;[1 0 0] Event Tick
  (`parent.ReceiveTick` DeltaSeconds)
  (`|ExecutionSequence`
    (:`then_0`
      ;[1 1 1] If slimed -> run faster
      (if (not (and (== (`self.SlimeAmountNormal`) 0) (== (`self.SlimeAmountPoison`) 0)))
        (set `CharacterMovementComponent.MaxWalkSpeed` (`self.RunSpeed`) (`self.CharacterMovement`))))
    (:`then_1`
      ;[1 1 1] Update Sickness
      (`HealthComponent.UpdateSickness` (`self.Health`) (`self.SlimeAmountNormal`) (`self.SlimeAmountPoison`)))))

(fn `UserConstructionScript`
  (`parent.UserConstructionScript`))