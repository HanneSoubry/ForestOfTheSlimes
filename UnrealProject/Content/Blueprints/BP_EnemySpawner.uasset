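; BP_EnemySpawner spawns a set number of slime enemies at its own location, one each time a delay timer elapses.
; Tick advances the timer and, when it fires, spawns either a base or poisonous slime AI based on the Type setting, then resets.
; An optional wall requirement holds spawning back until a WallDown event arrives with the matching wall ID.
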(event `self.ReceiveTick`
  (params (DeltaSeconds :type "Float (single-precision)"))
  (bind _defaultsceneroot (`self.DefaultSceneRoot`))
  (bind _returnvalue (`SceneComponent.K2_GetComponentLocation` _defaultsceneroot))
  (bind _returnvalue_2 (`SceneComponent.K2_GetComponentRotation` _defaultsceneroot))
  (if (not (`self.WallRequirement`))
    ;[1 1 1] If more should spawn
    (if (< (`self.AmountSpawned`) (`self.Amount`))
      ;[1 1 1] Increase current timer
      (bind _output_get (set `self.CurrentTime` (+ (`self.CurrentTime`) DeltaSeconds)))
      ;[1 1 1] If time to spawn
      (if (>= _output_get (`self.DelayTime`))
        ;[1 1 1] Increase nr spawned
        (set `self.AmountSpawned` (+ (`self.AmountSpawned`) 1))
        ;[1 1 1] Spawn enemy
        (switch `/Game/Blueprints/Enum_SlimeType` (`self.Type`)
          (:`NewEnumerator0`
            (`AIBlueprintHelperLibrary.SpawnAIFromClass` "/Game/Blueprints/BP_BaseSlime.BP_BaseSlime_C" null _returnvalue _returnvalue_2 false null))
          (:`NewEnumerator1`
            (`AIBlueprintHelperLibrary.SpawnAIFromClass` "/Game/Blueprints/BP_SlimePoisonous.BP_SlimePoisonous_C" null _returnvalue _returnvalue_2 false null)))
        ;[1 1 1] Reset timer
        (set `self.CurrentTime` 0.0)))))

(event `WallDown`
  (params (ID :type Integer))
  ;[1 1 1] If required wall is down
  (if (`self.WallRequirement`)
    (if (== ID (`self.Wall_ID`))
      (set `self.WallRequirement` false))))

(fn `UserConstructionScript`)