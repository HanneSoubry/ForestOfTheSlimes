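; Game state for the slime game that tracks the current level number and run timer and handles level completion and failure.
; The level number is parsed from the map name, and Tick accumulates time, exposed as minutes and seconds by GetTimer.
; Reaching the goal saves the time through the game mode, shows the end screen and, before the last level, increments the level and resets player health parameters.
; Failing stops the timer and shows the failure screen.
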(event `self.ReceiveBeginPlay`
  ;[1 1 1] Find current level nr
  (bind _returnvalue (`GameplayStatics.GetCurrentLevelName` true))
  (set `self.LevelNr` (`KismetStringLibrary.Conv_StringToInt` (`.RightS` (`KismetStringLibrary.Split` _returnvalue "Level")))))

(event `GoalReached`
  (bind _levelnr (`self.LevelNr`))
  ;[1 1 1] Goal reached
  (set `self.StopTimer` true)
  ;[1 1 1] Save game info
  (bind _asbp_slime_game_mode (cast `/Game/Blueprints/BP_SlimeGameMode` (`GameplayStatics.GetGameMode`))
    (:`then`
      ;;[1 1 1] Set variables
      (`/Game/Blueprints/BP_SlimeSaveGame.SaveTime` (`/Game/Blueprints/BP_SlimeGameMode.SaveGameInstance` _asbp_slime_game_mode) (`self.LevelNr`) (`self.LevelTimer`))
      ;;[1 1 1] Push to save file
      (`/Game/Blueprints/BP_SlimeGameMode.Save Game` _asbp_slime_game_mode))
    (:`CastFailed`
      _))
  ;[1 1 1] Check levelNr
  (if (< _levelnr (`self.MaxLevel`))
    ;[1 1 1] Increase LevelNr
    (set `self.LevelNr` (+ _levelnr 1))
    ;[1 1 1] Next level
    (`WidgetLayoutLibrary.RemoveAllWidgets`)
    (bind _returnvalue (`|CreateWidget` "/Game/Blueprints/BPW_EndScreen.BPW_EndScreen_C"))
    (`UserWidget.AddToViewport` _returnvalue 0)
    (set `/Game/Blueprints/BPW_EndScreen.LevelCompeted` true _returnvalue)
    (set `/Game/Blueprints/BPW_EndScreen.FinalLevel` false _returnvalue)
    ;[1 1 1] Set Level start parameters
    (bind _returnvalue_2 (`GameplayStatics.GetActorOfClass` "/Game/Blueprints/BP_StartParams.BP_StartParams_C"))
    (bind _asbp_player_character (cast `/Game/Blueprints/BP_PlayerCharacter` (`GameplayStatics.GetPlayerPawn` 0)))
    (`HealthComponent.InitializeParams` (`/Game/Blueprints/BP_PlayerCharacter.Health` _asbp_player_character) (`/Game/Blueprints/BP_StartParams.MaxHealth` _returnvalue_2) (`/Game/Blueprints/BP_StartParams.MaxSickness` _returnvalue_2))
    (else
      ;[1 1 1] Last level completed
      (`WidgetLayoutLibrary.RemoveAllWidgets`)
      (bind _returnvalue_3 (`|CreateWidget` "/Game/Blueprints/BPW_EndScreen.BPW_EndScreen_C"))
      (`UserWidget.AddToViewport` _returnvalue_3 0)
      (set `/Game/Blueprints/BPW_EndScreen.LevelCompeted` true _returnvalue_3)
      (set `/Game/Blueprints/BPW_EndScreen.FinalLevel` true _returnvalue_3))))

(event `FailedLevel`
  ;[1 1 1] Failed Level
  (set `self.StopTimer` true)
  (`WidgetLayoutLibrary.RemoveAllWidgets`)
  (bind _returnvalue (`|CreateWidget` "/Game/Blueprints/BPW_EndScreen.BPW_EndScreen_C"))
  (set `/Game/Blueprints/BPW_EndScreen.LevelCompeted` false _returnvalue)
  (`UserWidget.AddToViewport` _returnvalue 0))

(event `self.ReceiveTick`
  (params (DeltaSeconds :type "Float (single-precision)"))
  (if (not (`self.StopTimer`))
    ;[1 1 1] Update timer
    (set `self.LevelTimer` (+ DeltaSeconds (`self.LevelTimer`)))))

(fn `GetTimer`
  (returns (Minutes :type Integer) (Seconds :type Integer))
  (bind _returnvalue (`KismetMathLibrary.FFloor` (`self.LevelTimer`)))
  (bind _returnvalue_2 (/ _returnvalue 60))
  (return _returnvalue_2 (- _returnvalue (* _returnvalue_2 60))))

(fn `UserConstructionScript`)