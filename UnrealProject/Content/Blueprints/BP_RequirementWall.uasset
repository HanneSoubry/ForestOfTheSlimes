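; BP_RequirementWall is a barrier that lowers out of the way once players supply enough slime to meet its requirement.
; DecreaseSlime subtracts from the clamped requirement and updates a "Slime left" text display.
; At zero it disables the cube's collision, reports its ID to BP_SlimeGameMode via WallDown, and starts moving.
; Tick then slides the actor down at a set speed until it covers the target distance.
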(event `self.ReceiveBeginPlay`
  ;[1 1 1] Set start text
  (`TextRenderComponent.K2_SetText` (`self.SlimeLeftText`) (`KismetTextLibrary.Conv_StringToText` (`KismetStringLibrary.Concat_StrStr` "Slime left : " (`KismetStringLibrary.Conv_IntToString` (`self.SlimeRequirement`))))))

(event `DecreaseSlime`
  (params (slimeAmount :type Integer))
  ;[1 1 1] if requirement not fulfilled yet
  (if (> (`self.SlimeRequirement`) 0)
    ;[1 1 1] Decrease slime
    (bind _output_get (set `self.SlimeRequirement` (`KismetMathLibrary.Clamp` (- (`self.SlimeRequirement`) slimeAmount) 0 100)))
    (`TextRenderComponent.K2_SetText` (`self.SlimeLeftText`) (`KismetTextLibrary.Conv_StringToText` (`KismetStringLibrary.Concat_StrStr` "Slime left : " (`KismetStringLibrary.Conv_IntToString` _output_get))))
    ;[1 1 1] If now fulfilled, start moving
    (if (== (`self.SlimeRequirement`) 0)
      (set `self.Moving` true)
      (`PrimitiveComponent.SetCollisionEnabled` (`self.Cube`) "NoCollision")
      ;[1 1 1] Pass wall ID to game mode
      (bind _asbp_slime_game_mode (cast `/Game/Blueprints/BP_SlimeGameMode` (`GameplayStatics.GetGameMode`)))
      (`/Game/Blueprints/BP_SlimeGameMode.WallDown` _asbp_slime_game_mode (`self.ID`)))))

(event `self.ReceiveTick`
  (params (DeltaSeconds :type "Float (single-precision)"))
  (bind (_returnvalue_x _returnvalue_y _returnvalue_z) (`KismetMathLibrary.BreakVector` (`self.K2_GetActorLocation`)))
  (bind _returnvalue (* (`self.Speed`) DeltaSeconds))
  (if (`self.Moving`)
    ;[1 1 1] Move
    (`self.K2_SetActorLocation` (`KismetMathLibrary.MakeVector` _returnvalue_x _returnvalue_y (- _returnvalue_z _returnvalue)))
    (bind _output_get (set `self.DistanceDone` (+ _returnvalue (`self.DistanceDone`))))
    (if (>= _output_get (`self.TargetDistance`))
      (set `self.Moving` false))))

(fn `UserConstructionScript`)